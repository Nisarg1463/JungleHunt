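; BP_FirePatch is a fire patch actor that keeps turning to face the player character.
; Each Tick it applies a look-at rotation toward player 0 and hides itself beyond a fixed distance from them.
; When its Center component overlaps another fire patch it compares Priority values, but the result does nothing because the DestroyActor call is disconnected.
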(event OnComponentBeginOverlap(Center)
  (params (OverlappedComponent :type Primitive%20Component%20Object%20Reference) (OtherActor :type Actor%20Object%20Reference) (OtherComp :type Primitive%20Component%20Object%20Reference) (OtherBodyIndex :type Integer) (bFromSweep :type Boolean) (SweepResult :type Hit%20Result%20Structure%20%28by%20ref%29))
  (if (== (Utilities|GetClass OtherActor) "BP_FirePatch_C")
    (bind _asbp_fire_patch (Utilities|Casting|CastToBP_FirePatch OtherActor))
    (if (> (Variables|BP_FirePatch_C|GetPriority _asbp_fire_patch) (Variables|Default|GetPriority))
      _)))

(event EventBeginPlay)

(event EventTick
  (params (DeltaSeconds :type Float%20%28single-precision%29))
  (bind _returnvalue (Game|GetPlayerCharacter 0))
  (bind _returnvalue_2 (Transformation|GetActorLocation))
  (bind _returnvalue_3 (Transformation|GetActorLocation _returnvalue))
  (Transformation|SetActorRotation (Math|Rotator|FindLookatRotation _returnvalue_2 _returnvalue_3))
  (Rendering|SetActorHiddenInGame (> (Math|Vector|Distance(Vector) _returnvalue_2 _returnvalue_3) 5.5e+03)))

(fn ConstructionScript)