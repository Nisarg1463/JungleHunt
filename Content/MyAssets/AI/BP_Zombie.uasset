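; Zombie AI character that chases and attacks players and dies when its health runs out.
; Perception updates toggle players in a target list, setting the current target, movement speed and Blackboard keys for sighting.
; A looping timer, started on BeginPlay and reset on player collisions, runs a range-checked attack montage, followed by a delayed trace between two arrows to apply damage.
; Taking lethal damage plays the dying animation and flags the Blackboard as dead.
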(event OnComponentHit(CapsuleComponent)
  (params (HitComponent :type Primitive%20Component%20Object%20Reference) (OtherActor :type Actor%20Object%20Reference) (OtherComp :type Primitive%20Component%20Object%20Reference) (NormalImpulse :type Vector :default "0, 0, 0") (Hit :type Hit%20Result%20Structure%20%28by%20ref%29))
  (Collision|SetCollisionResponsetoChannel (Variables|Character|GetMesh) "ECC_GameTraceChannel2" "ECR_Ignore")
  (Utilities|Time|ClearandInvalidateTimerbyHandle (stale _returnvalue))
  (CallFunction|Attack)
  (if (== (Utilities|GetClass OtherActor) "/Game/MyAssets/Animations/Player/BP_Player.BP_Player_C")
    (bind _returnvalue (Utilities|Time|SetTimerbyEvent (delegate Custom|Attack) 3.0 true))))

(event OnTargetPerceptionUpdated(AIPerception)
  (params (Actor :type Actor%20Object%20Reference) (Stimulus :type AI%20Stimulus%20Structure))
  (bind _players (Variables|Default|GetPlayers))
  (Variables|Default|SetFound false)
  (bind (_array_element _array_index) (Utilities|Array|ForEachLoopwithBreak (Variables|Default|GetPlayers) :!label _label)
    (:LoopBody
      (if (== _array_element Actor)
        (Utilities|Array|RemoveIndex (Variables|Default|GetPlayers) _array_index)
        (if (> (Utilities|Array|Length _players) 0)
          (Variables|Default|SetPlayer (Utilities|Array|Get(acopy) _players))
          (AI|Components|Blackboard|SetValueasBool (AI|GetBlackboard (AI|GetAIController self)) (Utilities|Name|MakeLiteralName "HasSeenPlayer") true)
          (Variables|/Script/Engine.CharacterMovementComponent|SetMaxWalkSpeed (Variables|Character|GetCharacterMovement) 4e+02)
          (else
            (AI|Components|Blackboard|SetValueasBool (AI|GetBlackboard (AI|GetAIController self)) (Utilities|Name|MakeLiteralName "HasSeenPlayer") false)
            (Variables|/Script/Engine.CharacterMovementComponent|SetMaxWalkSpeed (Variables|Character|GetCharacterMovement) 2e+02)
            (Variables|Default|SetFollowing false)))
        (Variables|Default|SetFound true)
        (goto _label Break)))
    (:Completed
      (if (not (Variables|Default|GetFound))
        (bind _asbp_player (Utilities|Casting|CastToBP_Player Actor))
        (bind _output_get (Variables|Default|SetPlayer _asbp_player))
        (Utilities|Array|Add (Variables|Default|GetPlayers) _output_get)
        (AI|Components|Blackboard|SetValueasBool (AI|GetBlackboard (AI|GetAIController self)) (Utilities|Name|MakeLiteralName "HasSeenPlayer") true)
        (Variables|/Script/Engine.CharacterMovementComponent|SetMaxWalkSpeed (Variables|Character|GetCharacterMovement) 4e+02)
        (Variables|Default|SetFollowing true)))))

(event Custom|Attack
  (bind _players (Variables|Default|GetPlayers))
  (if (Variables|Default|GetFollowing)
    (if (< (Math|Vector|Distance(Vector) (Transformation|GetActorLocation (Variables|Default|GetPlayer)) (Transformation|GetActorLocation self)) 1.5e+02)
      (Animation|PlayAnimMontage "/Game/MyAssets/Animations/Zombie/AM_Attack.AM_Attack" 1.0 "None")
      (CallFunction|DamagePlayer)
      (if (<= (Variables|/Game/MyAssets/Animations/Player/BP_Player.BP_Player_C|GetHealth (Variables|Default|GetPlayer)) 0.0)
        (Utilities|Array|RemoveItem (Variables|Default|GetPlayers) (Variables|Default|GetPlayer))
        (if (> (Utilities|Array|Length _players) 0)
          (Variables|Default|SetPlayer (Utilities|Array|Get(acopy) _players))
          (AI|Components|Blackboard|SetValueasBool (AI|GetBlackboard (AI|GetAIController self)) (Utilities|Name|MakeLiteralName "HasSeenPlayer") true)
          (Variables|/Script/Engine.CharacterMovementComponent|SetMaxWalkSpeed (Variables|Character|GetCharacterMovement) 4e+02)
          (else
            (AI|Components|Blackboard|SetValueasBool (AI|GetBlackboard (AI|GetAIController self)) (Utilities|Name|MakeLiteralName "HasSeenPlayer") false)
            (Variables|/Script/Engine.CharacterMovementComponent|SetMaxWalkSpeed (Variables|Character|GetCharacterMovement) 2e+02)
            (Variables|Default|SetFollowing false)))
        (Variables|Default|SetFound true)
        (Utilities|Array|ForEachLoopwithBreak (Variables|Default|GetPlayers)) ; enters at Break
        (else
          (Variables|/Script/Engine.CharacterMovementComponent|SetMaxWalkSpeed (Variables|Character|GetCharacterMovement) (Class|MovementComponent|GetMaxSpeed (Variables|/Script/Engine.Character|GetCharacterMovement (Variables|Default|GetPlayer))))))
      (else
        (Variables|/Script/Engine.CharacterMovementComponent|SetMaxWalkSpeed (Variables|Character|GetCharacterMovement) 4e+02)))))

(event Custom|DamagePlayer
  (Utilities|FlowControl|Delay 1.5)
  (bind _outhit (Collision|LineTraceByChannel (Transformation|GetSocketLocation (Variables|Default|GetArrow1) "None") (Transformation|GetSocketLocation (Variables|Default|GetArrow2) "None") "TraceTypeQuery3" false (Utilities|Array|MakeArray (Components|GetOwner)) "None"))
  (if (== (Utilities|GetClass (.hitactor _outhit)) "/Game/MyAssets/Animations/Player/BP_Player.BP_Player_C")
    (bind _asbp_player (Utilities|Casting|CastToBP_Player (.hitactor _outhit)))
    (Default|Hit _asbp_player (Variables|Default|GetDamage))))

(event EventBeginPlay
  (bind _returnvalue (Utilities|Time|SetTimerbyEvent (delegate Custom|Attack) 3.0 true)))

(fn ConstructionScript)

(fn Hit
  (params (Damage :type Float%20%28double-precision%29))
  (bind _output_get (Variables|Default|SetHealth (- (Variables|Default|GetHealth) Damage)))
  (if (<= _output_get 0.0)
    (Variables|Default|SetIsDead true)
    (Components|Animation|PlayAnimation (Variables|Character|GetMesh) "/Game/MyAssets/Animations/Zombie/Zombie_Dying_mixamo_com.Zombie_Dying_mixamo_com" false)
    (AI|Components|Blackboard|SetValueasBool (AI|GetBlackboard (AI|GetAIController self)) (Utilities|Name|MakeLiteralName "Dead") true)))

(fn SetSpeed
  (params (Speed :type Float%20%28double-precision%29))
  (Variables|/Script/Engine.CharacterMovementComponent|SetMaxWalkSpeed (Variables|Character|GetCharacterMovement) Speed))